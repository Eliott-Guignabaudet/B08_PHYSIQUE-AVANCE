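; BP_Projectile is a physics-driven projectile for FurieuxOiseaux that previews its trajectory, launches, and explodes on impact.
; PredictTrajectory debug-draws the predicted path each call, using the same direction, force and multiplier velocity as Launch.
; Launch detaches the Collider to absolute location, enables physics and gravity, then applies a velocity-change impulse.
; The first hit on anything except the pawn or another projectile spawns a Niagara explosion, removes the components, then destroys the actor after a delay.
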(event `self.Collider.OnComponentHit`
  (params (HitComponent :type "PrimitiveComponent Object Reference") (OtherActor :type "Actor Object Reference") (OtherComp :type "PrimitiveComponent Object Reference") (NormalImpulse :type "Vector Structure") (Hit :type "HitResult Structure (by ref)"))
  (bind _returnvalue (`GameplayStatics.GetObjectClass` OtherActor))
  (if (not (or (== _returnvalue "/Game/Developers/Cheetoh/Collections/BP_FurieuxOiseauxPawn.BP_FurieuxOiseauxPawn_C") (== _returnvalue "BP_Projectile_C") (`self.bHaveHit`)))
    (bind _returnvalue_2 (`NiagaraFunctionLibrary.SpawnSystemAtLocation` "/Game/FurieuxOiseaux/Blueprints/Actors/Projectiles/NS_ProjectileExplosion.NS_ProjectileExplosion" (`SceneComponent.K2_GetComponentLocation` (`self.Collider`)) (struct) (2.0 2.0 2.0)))
    (set `self.bHaveHit` true)
    (`ActorComponent.K2_DestroyComponent` (`self.Sphere`))
    (`ActorComponent.K2_DestroyComponent` (`self.Collider`))
    (`KismetSystemLibrary.Delay` 2.0)
    (`ActorComponent.K2_DestroyComponent` _returnvalue_2)
    (`self.K2_DestroyActor`)))

(event `ProjectileInterface.PredictTrajectory`
  (params (DirectionValue :type "Vector Structure") (ForceValue :type "Float (single-precision)"))
  (`GameplayStatics.Blueprint_PredictProjectilePath_Advanced` (make `PredictProjectilePathParams` (`SceneComponent.K2_GetComponentLocation` (`self.Sphere`)) (* DirectionValue ForceValue (`self.ForceMultiplier`)) false 20.0 1.0 true "ECC_WorldStatic" (`|MakeArray` "ObjectTypeQuery1" :!type "EObjectTypeQuery Enum") _ 20.0 0.0 "ForOneFrame")))

(event `ProjectileInterface.Launch`
  (params (DirectionValue :type "Vector Structure") (ForceValue :type "Float (single-precision)"))
  (bind _collider (`self.Collider`))
  (`PrimitiveComponent.SetSimulatePhysics` _collider true)
  (`PrimitiveComponent.SetEnableGravity` _collider true)
  (set `SceneComponent.bAbsoluteLocation` true _collider)
  (`SceneComponent.K2_SetRelativeLocation` _collider (`self.K2_GetActorLocation`) false true)
  (`PrimitiveComponent.AddImpulse` (`self.Collider`) (* DirectionValue ForceValue (`self.ForceMultiplier`)) "None" true))

(fn `UserConstructionScript`)