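; BP_Enemy is a destructible enemy in the FurieuxOiseaux game that takes damage from physical impacts.
; It sets its health on BeginPlay, then listens for hits on its static mesh.
; Hits whose normal impulse reaches a threshold subtract health in proportion to impulse strength, truncated to a whole number.
; The actor destroys itself when health reaches zero or below.
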(event `self.ReceiveBeginPlay`
  (set `self.Health` 300))

(event `self.StaticMeshComponent.OnComponentHit`
  (params (HitComponent :type "PrimitiveComponent Object Reference") (OtherActor :type "Actor Object Reference") (OtherComp :type "PrimitiveComponent Object Reference") (NormalImpulse :type "Vector Structure") (Hit :type "HitResult Structure (by ref)"))
  (bind _returnvalue (`KismetMathLibrary.VSize` NormalImpulse))
  (if (>= _returnvalue 50000.0)
    (bind _output_get (set `self.Health` (`KismetMathLibrary.FTrunc` (- (`self.Health`) (/ _returnvalue 50000.0)))))
    (if (<= _output_get 0)
      (`self.K2_DestroyActor`))))

(fn `UserConstructionScript`)