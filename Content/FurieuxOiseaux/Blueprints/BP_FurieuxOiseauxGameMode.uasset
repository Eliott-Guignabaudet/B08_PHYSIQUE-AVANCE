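; Game mode for FurieuxOiseaux that tracks the total score and ends the game once every enemy is dead.
; On BeginPlay it finds all BP_Enemy actors, binds AddToTotalScore to their AddToScore event and stores their count.
; Each callback adds the enemy's death score and decrements the count, calling EndGame at zero.
; EndGame is a placeholder that only prints a French end-of-game screen message.
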(event `self.ReceiveBeginPlay`
  (bind _outactors (`GameplayStatics.GetAllActorsOfClass` "/Game/FurieuxOiseaux/Blueprints/BP_Enemy.BP_Enemy_C"))
  (add `/Game/FurieuxOiseaux/Blueprints/BP_Enemy.AddScore` _outactors (delegate `AddToTotalScore`))
  (set `self.NumberOfEnemies` (`KismetArrayLibrary.Array_Length` _outactors)))

(event `AddToTotalScore`
  (set `self.TotalScore` (+ (`self.EnemyDeathScore`) (`self.TotalScore`)))
  (bind _output_get (set `self.NumberOfEnemies` (- (`self.NumberOfEnemies`) 1)))
  (if (<= _output_get 0)
    (`self.EndGame`)))

(fn `EndGame`
  (`KismetSystemLibrary.PrintString` "Écran de fin de jeu" true true (struct :`G` 0.66 :`B` 1.0 :`A` 1.0) 10000.0))

(fn `UserConstructionScript`)